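; BP_Grid is a tactical movement grid that builds tiles from the level and finds paths for the selected unit.
; Sphere traces classify cells by ground and obstacle type into a tile map, previewed as debug planes in construction and spawned as BP_GridTile actors on BeginPlay.
; Hovering runs four-way weighted A* and highlights the path, capped at the unit's Mp in tile count.
; Selecting passes that path to the player controller unless a unit is moving.
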(event Custom|Event_NewTileSelected
  (params (selectedTile :type BP%20Grid%20Tile%20Object%20Reference))
  (Utilities|IsValid (Variables|Grid|GetselectedTile)
    (:Is%20Valid
      (Default|EventDeselectTile (Variables|Grid|GetselectedTile)))
    (:Is%20Not%20Valid
      _))
  (Variables|Grid|SetselectedTile selectedTile)
  (if (not (Variables|Default|GetisAUnitMoving))
    (Default|EventNewPathAvailable (Variables|Default|GetplayerController) (Variables|Default|Getpath))))

(event Custom|Event_NewTileHovered
  (params (hoveredTile :type BP%20Grid%20Tile%20Object%20Reference))
  (bind _playercontroller (Variables|Default|GetplayerController))
  (bind _selectedunit (Variables|/Game/Blueprints/Controllers/BP_PlayerController.BP_PlayerController_C|GetSelectedUnit _playercontroller))
  (Utilities|IsValid (Variables|Grid|GethoveredTile)
    (:Is%20Valid
      (Default|EventEndHoverTile (Variables|Grid|GethoveredTile)))
    (:Is%20Not%20Valid
      _))
  (Variables|Grid|SethoveredTile hoveredTile)
  (CallFunction|HighlightCurrentPath false)
  (if (Math|Boolean|ANDBoolean (Utilities|IsValid _selectedunit) (Utilities|IsValid (Variables|Grid|GethoveredTile)) (not (Variables|Default|GetisAUnitMoving)))
    (Pathfinding|FindPathtoTarget (Variables|/Game/Blueprints/Controllers/BP_Unit.BP_Unit_C|GetgridIndex _selectedunit) (Variables|/Game/Blueprints/Grid/BP_GridTile.BP_GridTile_C|GetGridIndex (Variables|Grid|GethoveredTile)))
    (CallFunction|HighlightCurrentPath true)))

(event EventBeginPlay
  (Rendering|Debug|FlushPersistentDebugLines)
  (Variables|Grid|SetGridLocation (Transformation|GetWorldLocation (Variables|Default|GetScene)))
  (Grid|GenerateMapDatafromWorld)
  (Grid|SpawnTile false)
  (Variables|Default|SetplayerController (.AsBP%20Player%20Controller (Utilities|Casting|CastToBP_PlayerController (Game|GetPlayerController 0)))))

(fn ConstructionScript
  (bind _gridsizeworld (Variables|Grid|GetGridSizeWorld))
  (Rendering|Debug|FlushPersistentDebugLines)
  (Variables|Grid|SetGridLocation (Transformation|GetWorldLocation (Variables|Default|GetScene)))
  (Rendering|Debug|DrawDebugBox (Variables|Grid|GetGridLocation) (Math|Vector|MakeVector (.y _gridsizeworld) (.x _gridsizeworld) 5.0) (Variables|Debug|GetGridColor) "0, 0, 0" 1.5908979977337438e+19 1e+01)
  (Rendering|Debug|DrawDebugBox (Grid|GridBottomLeft) (Math|Vector|MakeVector 2e+01 2e+01 2e+01) (Variables|Debug|GetBottomLeftColor) "0, 0, 0" 1.5908979977337438e+19 1e+01)
  (Grid|GenerateMapDatafromWorld)
  (Debug|DrawTile))

(fn GridBottomLeft
  (return (- (- (Variables|Grid|GetGridLocation) (* (Math|Vector|GetRightVector (Variables|Default|GetScene)) (.x (Variables|Grid|GetGridSizeWorld)))) (* (Math|Vector|GetForwardVector (Variables|Default|GetScene)) (.y (Variables|Grid|GetGridSizeWorld))))))

(fn GridTileNumber
  (bind _gridsizeworld (Variables|Grid|GetGridSizeWorld))
  (bind _tilesize (Variables|Grid|GetTileSize))
  (bind _returnvalue (/ _gridsizeworld _tilesize))
  (return (- (Math|Float|Floor (.x _returnvalue)) 1) (- (Math|Float|Floor (.y _returnvalue)) 1)))

(fn DrawTile
  (bind _keys (Utilities|Map|Keys (Variables|Grid|Getstruct_Tiles)))
  (for _array_element _keys
    (Debug|DrawDebugPlane (.worldlocation (.Value (Utilities|Map|Find (Variables|Grid|Getstruct_Tiles) _array_element))) (.groundtype (.Value (Utilities|Map|Find (Variables|Grid|Getstruct_Tiles) _array_element))))))

(fn SphereTraces
  (params (Location :type Vector) (TraceChannel :type ETraceTypeQuery%20Enum :default "TraceTypeQuery1"))
  (bind (_outhit _returnvalue) (Collision|SphereTraceByChannel Location Location (- (Variables|Grid|GetTileSize) (Variables|Grid|GetTileSizeMinus)) TraceChannel false 0 "None" true "(R=1.000000,G=0.000000,B=0.000000,A=1.000000)" "(R=0.000000,G=1.000000,B=0.000000,A=1.000000)" 2e+01))
  (return _returnvalue (.hitactor _outhit)))

(fn DrawDebugPlane
  (params (Location :type Vector) (GroundType :type Enum_GroundTypes%20Enum :default "NewEnumerator0"))
  (bind _z (Math|Vector|BreakVector Location))
  (bind _tilesize (Variables|Grid|GetTileSize))
  (bind _tilesizeminus (Variables|Grid|GetTileSizeMinus))
  (bind _returnvalue (- _tilesize _tilesizeminus))
  (switch Utilities|FlowControl|Switch|SwitchonEnum_GroundTypes GroundType
    (:NewEnumerator0
      (Class|KismetSystemLibrary|DrawDebugPlane (Utilities|Struct|MakePlane _z 0.0 0.0 1.0) Location _returnvalue "(R=0.990218,G=1.000000,B=0.440498,A=1.000000)" 11111110656.0))
    (:NewEnumerator1
      (Class|KismetSystemLibrary|DrawDebugPlane (Utilities|Struct|MakePlane _z 0.0 0.0 1.0) Location _returnvalue "(R=1.000000,G=0.436468,B=0.000000,A=1.000000)" 11111110656.0))
    (:NewEnumerator2
      (Class|KismetSystemLibrary|DrawDebugPlane (Utilities|Struct|MakePlane _z 0.0 0.0 1.0) Location _returnvalue "(R=1.000000,G=0.009182,B=0.000000,A=1.000000)" 11111110656.0))))

(fn GenerateMapDatafromWorld
  (bind (_gridtilenbx _gridtilenby) (Grid|GridTileNumber))
  (bind _tilesize (Variables|Grid|GetTileSize))
  (bind _tilesize_2 (Variables|Grid|GetTileSize))
  (for _index (range 0 _gridtilenbx)
    (LocalVariables|SetX _index)
    (for _index_2 (range 0 _gridtilenby)
      (LocalVariables|SetY _index_2)
      (LocalVariables|SetTilePosition (+ (Grid|GridBottomLeft) (* (Math|Vector|GetRightVector (Variables|Default|GetScene)) (+ (* (LocalVariables|GetX) (* _tilesize_2 2.0)) _tilesize_2)) (* (Math|Vector|GetForwardVector (Variables|Default|GetScene)) (+ (* (LocalVariables|GetY) (* _tilesize 2.0)) _tilesize))))
      (if (.HitSomething (Grid|SphereTraces (LocalVariables|GetTilePosition) "TraceTypeQuery3"))
        (if (.HitSomething (Grid|SphereTraces (LocalVariables|GetTilePosition) "TraceTypeQuery4"))
          (Utilities|Map|Add (Variables|Grid|Getstruct_Tiles) (Math|Vector2D|MakeVector2D (Math|Conversions|ToFloat(Integer) (LocalVariables|GetX)) (Math|Conversions|ToFloat(Integer) (LocalVariables|GetY))) (Utilities|Struct|MakeStruct_Tiles 0 0 (Variables|/Game/Blueprints/Grid/BP_Base_Obstacle.BP_Base_Obstacle_C|GetEnum_Ground8types (.AsBP%20Base%20Obstacle (Utilities|Casting|CastToBP_Base_Obstacle (.Actor (Grid|SphereTraces (LocalVariables|GetTilePosition) "TraceTypeQuery4"))))) (LocalVariables|GetTilePosition) (Math|Vector2D|MakeVector2D (Math|Conversions|ToFloat(Integer) (LocalVariables|GetX)) (Math|Conversions|ToFloat(Integer) (LocalVariables|GetY))) (Grid|GetTileCost (Variables|/Game/Blueprints/Grid/BP_Base_Obstacle.BP_Base_Obstacle_C|GetEnum_Ground8types (.AsBP%20Base%20Obstacle (Utilities|Casting|CastToBP_Base_Obstacle (.Actor (Grid|SphereTraces (LocalVariables|GetTilePosition) "TraceTypeQuery4")))))) 0 0 0 "(X=0.000000,Y=0.000000)"))
          (else
            (Utilities|Map|Add (Variables|Grid|Getstruct_Tiles) (Math|Vector2D|MakeVector2D (Math|Conversions|ToFloat(Integer) (LocalVariables|GetX)) (Math|Conversions|ToFloat(Integer) (LocalVariables|GetY))) (Utilities|Struct|MakeStruct_Tiles 0 0 "NewEnumerator0" (LocalVariables|GetTilePosition) (Math|Vector2D|MakeVector2D (Math|Conversions|ToFloat(Integer) (LocalVariables|GetX)) (Math|Conversions|ToFloat(Integer) (LocalVariables|GetY))) (Grid|GetTileCost "NewEnumerator0") 0 0 0 "(X=0.000000,Y=0.000000)"))
            (Utilities|Array|Add (Variables|Grid|GetgridTilesLocation) (LocalVariables|GetTilePosition))))
        (else
          (Utilities|Map|Add (Variables|Grid|Getstruct_Tiles) (Math|Vector2D|MakeVector2D (Math|Conversions|ToFloat(Integer) (LocalVariables|GetX)) (Math|Conversions|ToFloat(Integer) (LocalVariables|GetY))) (Utilities|Struct|MakeStruct_Tiles 0 0 "NewEnumerator3" (LocalVariables|GetTilePosition) (Math|Vector2D|MakeVector2D (Math|Conversions|ToFloat(Integer) (LocalVariables|GetX)) (Math|Conversions|ToFloat(Integer) (LocalVariables|GetY))) (Grid|GetTileCost "NewEnumerator3") 0 0 0 "(X=0.000000,Y=0.000000)")))))))

(fn SpawnTile
  (params (SpawnNoneTiles :type Boolean))
  (bind _struct_tiles (Variables|Grid|Getstruct_Tiles))
  (bind _keys (Utilities|Map|Keys (Variables|Grid|Getstruct_Tiles)))
  (for _array_element _keys
    (if (or SpawnNoneTiles (Utilities|Enum|NotEqual(Enum) (.groundtype (.Value (Utilities|Map|Find _struct_tiles _array_element))) "NewEnumerator3"))
      (bind _returnvalue (Game|SpawnActorfromClass "/Game/Blueprints/Grid/BP_GridTile.BP_GridTile_C" (Math|Transform|MakeTransform (.worldlocation (.Value (Utilities|Map|Find _struct_tiles _array_element))) (Transformation|GetWorldRotation (Variables|Default|GetScene)) "1,1,1") "Undefined" 0 0))
      (Variables|/Game/Blueprints/Grid/BP_GridTile.BP_GridTile_C|SetGridIndex _returnvalue _array_element)
      (Variables|/Game/Blueprints/Grid/BP_GridTile.BP_GridTile_C|Setbp_Grid _returnvalue self)
      (Utilities|Map|Add _struct_tiles _array_element (Utilities|Struct|MakeStruct_Tiles 0 _returnvalue (.groundtype (.Value (Utilities|Map|Find _struct_tiles _array_element))) (.worldlocation (.Value (Utilities|Map|Find _struct_tiles _array_element))) (.gridindex (.Value (Utilities|Map|Find _struct_tiles _array_element))) (.tilecost (.Value (Utilities|Map|Find _struct_tiles _array_element))) (.finalcost (.Value (Utilities|Map|Find _struct_tiles _array_element))) (.costfromstart (.Value (Utilities|Map|Find _struct_tiles _array_element))) (.estimatedcosttotarget (.Value (Utilities|Map|Find _struct_tiles _array_element))) (.previoustile (.Value (Utilities|Map|Find _struct_tiles _array_element))))))))

(fn GetTileCost
  (params (gridIndex :type Enum_GroundTypes%20Enum :default "NewEnumerator0"))
  (switch Utilities|FlowControl|Switch|SwitchonEnum_GroundTypes gridIndex
    (:NewEnumerator0
      (LocalVariables|SetCost 1))
    (:NewEnumerator1
      (LocalVariables|SetCost 3))
    (:NewEnumerator2
      (LocalVariables|SetCost 999 :!label _label))
    (:NewEnumerator3
      (goto _label)))
  (return (LocalVariables|GetCost)))

(fn GetTileNeighbours
  (params (gridIndex :type Vector%202D%20Structure))
  (bind _output_get (LocalVariables|SetpossibleNeighbours (Utilities|Array|MakeArray "(X=1.000000,Y=0.000000)" "(X=0.000000,Y=1.000000)" "(X=-1.000000,Y=0.000000)" "(X=0.000000,Y=-1.000000)")))
  (for _array_element _output_get
    (if (.ReturnValue (Utilities|Map|Find (Variables|Grid|Getstruct_Tiles) (+ _array_element gridIndex)))
      (if (Math|Boolean|ANDBoolean (== (.unitonthistile (.Value (Utilities|Map|Find (Variables|Grid|Getstruct_Tiles) (+ _array_element gridIndex)))) 0) (Utilities|Enum|NotEqual(Enum) (.groundtype (.Value (Utilities|Map|Find (Variables|Grid|Getstruct_Tiles) (+ _array_element gridIndex)))) "NewEnumerator2") (Utilities|Enum|NotEqual(Enum) (.groundtype (.Value (Utilities|Map|Find (Variables|Grid|Getstruct_Tiles) (+ _array_element gridIndex)))) "NewEnumerator3"))
        (Utilities|Array|AddUnique (LocalVariables|GetoutNeighbours) (+ _array_element gridIndex)))))
  (return (LocalVariables|GetoutNeighbours)))

(fn GetEstimatedCostTotarget
  (params (currentTile :type Vector%202D%20Structure) (targetTile :type Vector%202D%20Structure))
  (bind _returnvalue (- currentTile targetTile))
  (return (Math|Float|Round (+ (Math|Float|Absolute(Float) (.x _returnvalue)) (Math|Float|Absolute(Float) (.y _returnvalue))))))

(fn FindPathtoTarget
  (params (startTile :type Vector%202D%20Structure) (targetTile :type Vector%202D%20Structure))
  (bind _struct_tiles (Variables|Grid|Getstruct_Tiles))
  (bind _struct_tiles_2 (Variables|Grid|Getstruct_Tiles))
  (bind _struct_tiles_3 (Variables|Grid|Getstruct_Tiles))
  (bind _struct_tiles_4 (Variables|Grid|Getstruct_Tiles))
  (LocalVariables|SetstartTileL startTile)
  (LocalVariables|SettargetTileL targetTile)
  (Utilities|Array|Clear (Variables|Default|Getpath))
  (if (Math|Boolean|ANDBoolean (Utilities|Enum|NotEqual(Enum) (.groundtype (.Value (Utilities|Map|Find (Variables|Grid|Getstruct_Tiles) (LocalVariables|GettargetTileL)))) "NewEnumerator3") (.ReturnValue (Utilities|Map|Find (Variables|Grid|Getstruct_Tiles) (LocalVariables|GettargetTileL))) (Utilities|Enum|NotEqual(Enum) (.groundtype (.Value (Utilities|Map|Find (Variables|Grid|Getstruct_Tiles) (LocalVariables|GettargetTileL)))) "NewEnumerator2") (== (.unitonthistile (.Value (Utilities|Map|Find (Variables|Grid|Getstruct_Tiles) (LocalVariables|GettargetTileL)))) 0))
    (Utilities|FlowControl|Sequence
      (:then_0
        ;[1 1 1] Default Values Grid
        (bind _keys (Utilities|Map|Keys (Variables|Grid|Getstruct_Tiles)))
        (for _array_element _keys
          (Utilities|Map|Add _struct_tiles_4 _array_element (Utilities|Struct|MakeStruct_Tiles (.unitonthistile (.Value (Utilities|Map|Find _struct_tiles_4 _array_element))) (.tileactor (.Value (Utilities|Map|Find _struct_tiles_4 _array_element))) (.groundtype (.Value (Utilities|Map|Find _struct_tiles_4 _array_element))) (.worldlocation (.Value (Utilities|Map|Find _struct_tiles_4 _array_element))) (.gridindex (.Value (Utilities|Map|Find _struct_tiles_4 _array_element))) (.tilecost (.Value (Utilities|Map|Find _struct_tiles_4 _array_element))) 0 0 0 "(X=0.000000,Y=0.000000)")))
        (Utilities|Map|Add :TargetMap _struct_tiles :Value (Utilities|Struct|MakeStruct_Tiles (.unitonthistile (.Value (Utilities|Map|Find _struct_tiles (LocalVariables|GetstartTileL)))) (.tileactor (.Value (Utilities|Map|Find _struct_tiles (LocalVariables|GetstartTileL)))) (.groundtype (.Value (Utilities|Map|Find _struct_tiles (LocalVariables|GetstartTileL)))) (.worldlocation (.Value (Utilities|Map|Find _struct_tiles (LocalVariables|GetstartTileL)))) (.gridindex (.Value (Utilities|Map|Find _struct_tiles (LocalVariables|GetstartTileL)))) (.tilecost (.Value (Utilities|Map|Find _struct_tiles (LocalVariables|GetstartTileL)))) (Pathfinding|GetEstimatedCostTotarget (LocalVariables|GetstartTileL) (LocalVariables|GettargetTileL)) 0 (Pathfinding|GetEstimatedCostTotarget (LocalVariables|GetstartTileL) (LocalVariables|GettargetTileL)) "(X=0.000000,Y=0.000000)")))
      (:then_1
        (bind _output_get (LocalVariables|SetcurrentTile (LocalVariables|GetstartTileL)))
        (Utilities|Array|AddUnique (LocalVariables|GetopenSet) _output_get)
        (while (> (Utilities|Array|Length (LocalVariables|GetopenSet)) 0)
          (LocalVariables|SetopenSetCheapest (Utilities|Array|Get(acopy) (LocalVariables|GetopenSet)))
          (for _array_element_2 (LocalVariables|GetopenSet)
            ;[1 1 1] Set la tile la moins chère*
            (if (< (.finalcost (.Value (Utilities|Map|Find _struct_tiles_2 _array_element_2))) (.finalcost (.Value (Utilities|Map|Find _struct_tiles_2 (LocalVariables|GetopenSetCheapest)))))
              (LocalVariables|SetopenSetCheapest _array_element_2 :!label _label)
              (elif (== (.finalcost (.Value (Utilities|Map|Find _struct_tiles_2 _array_element_2))) (.finalcost (.Value (Utilities|Map|Find _struct_tiles_2 (LocalVariables|GetopenSetCheapest)))))
                (if (<= (.estimatedcosttotarget (.Value (Utilities|Map|Find _struct_tiles_2 _array_element_2))) (.estimatedcosttotarget (.Value (Utilities|Map|Find _struct_tiles_2 (LocalVariables|GetopenSetCheapest)))))
                  (goto _label)))))
          (LocalVariables|SetcurrentTile (LocalVariables|GetopenSetCheapest))
          (Utilities|Array|RemoveItem (LocalVariables|GetopenSet) (LocalVariables|GetcurrentTile))
          (Utilities|Array|AddUnique (LocalVariables|GetclosedSet) (LocalVariables|GetcurrentTile))
          (for _array_element_3 (Pathfinding|GetTileNeighbours (LocalVariables|GetcurrentTile))
            (LocalVariables|SetcurrentNeighbour _array_element_3)
            (if (not (Utilities|Array|ContainsItem (LocalVariables|GetclosedSet) (LocalVariables|GetcurrentNeighbour)))
              (LocalVariables|SetcurrentNeighouCostFromStart (+ (.costfromstart (.Value (Utilities|Map|Find (Variables|Grid|Getstruct_Tiles) (LocalVariables|GetcurrentTile)))) (.tilecost (.Value (Utilities|Map|Find (Variables|Grid|Getstruct_Tiles) (LocalVariables|GetcurrentNeighbour))))))
              (if (not (Utilities|Array|ContainsItem (LocalVariables|GetopenSet) (LocalVariables|GetcurrentNeighbour)))
                (Utilities|Array|AddUnique (LocalVariables|GetopenSet) (LocalVariables|GetcurrentNeighbour))
                (Utilities|Map|Add _struct_tiles_3 (LocalVariables|GetcurrentNeighbour) (Utilities|Struct|MakeStruct_Tiles (.unitonthistile (.Value (Utilities|Map|Find _struct_tiles_3 (LocalVariables|GetcurrentNeighbour)))) (.tileactor (.Value (Utilities|Map|Find _struct_tiles_3 (LocalVariables|GetcurrentNeighbour)))) (.groundtype (.Value (Utilities|Map|Find _struct_tiles_3 (LocalVariables|GetcurrentNeighbour)))) (.worldlocation (.Value (Utilities|Map|Find _struct_tiles_3 (LocalVariables|GetcurrentNeighbour)))) (.gridindex (.Value (Utilities|Map|Find _struct_tiles_3 (LocalVariables|GetcurrentNeighbour)))) (.tilecost (.Value (Utilities|Map|Find _struct_tiles_3 (LocalVariables|GetcurrentNeighbour)))) (+ (Pathfinding|GetEstimatedCostTotarget (LocalVariables|GetcurrentNeighbour) (LocalVariables|GettargetTileL)) (LocalVariables|GetcurrentNeighouCostFromStart)) (LocalVariables|GetcurrentNeighouCostFromStart) (Pathfinding|GetEstimatedCostTotarget (LocalVariables|GetcurrentNeighbour) (LocalVariables|GettargetTileL)) (LocalVariables|GetcurrentTile)) :!label _label_2)
                (if (Math|Vector|Equal(Vector) (LocalVariables|GetcurrentNeighbour) (LocalVariables|GettargetTileL) 0.0001)
                  (Variables|Default|Setpath (Pathfinding|RetracePath (LocalVariables|GettargetTileL) (LocalVariables|GetstartTileL)))
                  (return))
                (elif (< (LocalVariables|GetcurrentNeighouCostFromStart) (.costfromstart (.Value (Utilities|Map|Find _struct_tiles_3 (LocalVariables|GetcurrentNeighbour)))))
                  (goto _label_2))))))
        ;[1 1 1] Fail pas de chemn possible vers l'objectif
        (return)))))

(fn RetracePath
  (params (targetTile :type Vector%202D%20Structure) (startTile :type Vector%202D%20Structure))
  (LocalVariables|SetcurrentTile targetTile)
  (while (Math|Vector|NotEqual(Vector) (LocalVariables|GetcurrentTile) startTile 0.0001)
    (Utilities|Array|AddUnique (LocalVariables|GetreversedPath) (LocalVariables|GetcurrentTile))
    (LocalVariables|SetcurrentTile (.previoustile (.Value (Utilities|Map|Find (Variables|Grid|Getstruct_Tiles) (LocalVariables|GetcurrentTile))))))
  (bind (_arrayindex _arrayelement) (Utilities|Array|ReverseforEachLoop (LocalVariables|GetreversedPath))
    (:LoopBody
      (if (<= _arrayindex (- (Variables|/Game/Blueprints/Controllers/BP_Unit.BP_Unit_C|Getmp (Variables|/Game/Blueprints/Controllers/BP_PlayerController.BP_PlayerController_C|GetSelectedUnit (Variables|Default|GetplayerController))) 1))
        (Utilities|Array|AddUnique (LocalVariables|GetoutPath) _arrayelement)
        (else
          (return (LocalVariables|GetoutPath)))))
    (:Completed
      (return (LocalVariables|GetoutPath)))))

(fn HighlightCurrentPath
  (params (isForHighlight :type Boolean))
  (for _array_element (Variables|Default|Getpath)
    (Utilities|IsValid (.tileactor (.Value (Utilities|Map|Find (Variables|Grid|Getstruct_Tiles) _array_element)))
      (:Is%20Valid
        (Default|EventIsinPath (.tileactor (.Value (Utilities|Map|Find (Variables|Grid|Getstruct_Tiles) _array_element))) isForHighlight)))))