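; BP_GridTile is one clickable cell of BP_Grid, tinted by its ground type read from the grid's tile data.
; Cursor hover and click report to the grid, while hover, select and in-path events set flags and refresh the color.
; SetTileColor brightens hovered tiles, overrides path tiles in blue and drives material parameters for color and selection.
; After a short BeginPlay delay it also scales to the grid's tile size and feeds its W_TileCost widget.
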(event OnEndCursorOver(StaticMesh)
  (params (TouchedComponent :type Primitive%20Component%20Object%20Reference))
  (Default|EventNewTileHovered (Variables|grid|Getbp_Grid)))

(event OnBeginCursorOver(StaticMesh)
  (params (TouchedComponent :type Primitive%20Component%20Object%20Reference))
  (CallFunction|EventStartHoverTile)
  (Default|EventNewTileHovered (Variables|grid|Getbp_Grid) self))

(event OnClicked(StaticMesh)
  (params (TouchedComponent :type Primitive%20Component%20Object%20Reference) (ButtonPressed :type Key%20Structure))
  (CallFunction|EventSelectTile)
  (Default|EventNewTileSelected (Variables|grid|Getbp_Grid) self))

(event Custom|Event_DeselectTile
  (Variables|Grid|SetisSelected false)
  (Grid|SetTileColor))

(event Custom|Event_SelectTile
  (Variables|Grid|SetisSelected true)
  (Grid|SetTileColor))

(event Custom|Event_IsInPath
  (params (isInPath :type Boolean))
  (Variables|Grid|SetisInPath isInPath)
  (Grid|SetTileColor))

(event Custom|Event_EndHoverTile
  (Variables|Grid|SetisHovered false)
  (Grid|SetTileColor))

(event Custom|Event_StartHoverTile
  (Variables|Grid|SetisHovered true)
  (Grid|SetTileColor))

(event EventBeginPlay
  (Utilities|FlowControl|Delay 0.2)
  (Grid|SetTileColor)
  (Grid|SetTileSize)
  (CallFunction|SetWidgetVariables))

(fn ConstructionScript)

(fn SetTileColor
  (Utilities|FlowControl|Sequence
    (:then_0
      (switch Utilities|FlowControl|Switch|SwitchonEnum_GroundTypes (.groundtype (Grid|GetTileData))
        (:NewEnumerator0
          (LocalVariables|SettileColor "(R=0.772158,G=0.791667,B=0.573952,A=1.000000)"))
        (:NewEnumerator1
          (LocalVariables|SettileColor "(R=0.750000,G=0.306754,B=0.027344,A=1.000000)"))
        (:NewEnumerator2
          (LocalVariables|SettileColor "(R=1.000000,G=0.000000,B=0.007519,A=1.000000)"))
        (:NewEnumerator3
          (LocalVariables|SettileColor "(R=0.000000,G=0.000000,B=0.000000,A=0.000000)"))))
    (:then_1
      (if (Variables|Grid|GetisSelected)
        (Rendering|Material|SetScalarParameterValueonMaterials (Variables|Default|GetStaticMesh) "bIsSelected" 1.0)
        (else
          (Rendering|Material|SetScalarParameterValueonMaterials (Variables|Default|GetStaticMesh) "bIsSelected" 0.0))))
    (:then_2
      (if (Variables|Grid|GetisHovered)
        (LocalVariables|SettileColor (Math|Conversions|ToLinearColor(Vector) (* (Math|Conversions|ToVector(LinearColor) (LocalVariables|GettileColor)) 3.0)))))
    (:then_3
      (if (Variables|Grid|GetisInPath)
        (LocalVariables|SettileColor "(R=0.325494,G=0.376689,B=0.880208,A=0.384000)")))
    (:then_4
      ;[1 1 1] Set Color
      (Rendering|Material|SetVectorParameterValueonMaterials (Variables|Default|GetStaticMesh) "ColorTile" (Math|Conversions|ToVector(LinearColor) (LocalVariables|GettileColor))))))

(fn GetTileData
  (return (.Value (Utilities|Map|Find (Variables|/Game/Blueprints/Grid/BP_Grid.BP_Grid_C|Getstruct_Tiles (Variables|grid|Getbp_Grid)) (Variables|Grid|GetGridIndex)))))

(fn SetTileSize
  (bind _bp_grid (Variables|grid|Getbp_Grid))
  (bind _staticmesh (Variables|Default|GetStaticMesh))
  (bind _returnvalue (Transformation|GetWorldScale _staticmesh))
  (bind _tilesize (Variables|/Game/Blueprints/Grid/BP_Grid.BP_Grid_C|GetTileSize _bp_grid))
  (bind _returnvalue_2 (/ _tilesize 5e+01))
  (bind _returnvalue_3 (* _returnvalue _returnvalue_2))
  (Transformation|SetWorldScale3D _staticmesh (Math|Vector|MakeVector (.x _returnvalue_3) (.y _returnvalue_3) 1.0)))

(fn SetWidgetVariables
  (bind _widget (Variables|Default|GetWidget))
  (bind _returnvalue (UserInterface|GetUserWidgetObject _widget))
  (bind _asw_tile_cost (Utilities|Casting|CastToW_TileCost _returnvalue))
  (Variables|/Game/Blueprints/Grid/W_TileCost.W_TileCost_C|Setgrid _asw_tile_cost (Variables|grid|Getbp_Grid))
  (Variables|/Game/Blueprints/Grid/W_TileCost.W_TileCost_C|SetgridIndex _asw_tile_cost (Variables|Grid|GetGridIndex)))