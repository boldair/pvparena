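; Player controller for a grid-based game that tracks the selected unit and relays movement paths to it.
; Selection events deselect the previous unit and store the new one, while path events tell the current unit to move.
; On BeginPlay it caches the level's BP_Grid.
; The Q key runs a debug spawn that places a BP_Rogue on a random grid tile for each zero in a hardcoded list, printing progress.
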(event Custom|Event_NewUnitSelected
  (params (Unit :type BP%20Unit%20Object%20Reference))
  (Utilities|IsValid (Variables|Default|GetSelectedUnit)
    (:Is%20Valid
      (Default|EventDeselect (Variables|Default|GetSelectedUnit)))
    (:Is%20Not%20Valid
      _))
  (Variables|Default|SetSelectedUnit Unit))

(event Custom|Event_NewPathAvailable
  (params (path :type Array%20of%20Vector%202D%20Structures))
  (bind _selectedunit (Variables|Default|GetSelectedUnit))
  (Utilities|IsValid _selectedunit
    (:Is%20Valid
      (Default|EventMoveAlongthePath _selectedunit path))))

(event Custom|testSpawnCharacter
  (bind _returnvalue (Math|Random|RandomIntegerinRange 1 10))
  (bind _grid (Variables|Default|GetGrid))
  (bind _gridtileslocation (Variables|/Game/Blueprints/Grid/BP_Grid.BP_Grid_C|GetgridTilesLocation _grid))
  (bind _output (Utilities|Array|Get(acopy) _gridtileslocation _returnvalue))
  (Development|PrintString "Hello")
  (for _array_element (Utilities|Array|MakeArray 1 2 0 1)
    (if (== _array_element 0)
      (Development|PrintString (Utilities|String|ToString(Vector) _output) true true "(R=0.000000,G=0.660000,B=1.000000,A=1.000000)" 1e+02)
      (Game|SpawnActorfromClass "/Game/Blueprints/Controllers/BP_Rogue.BP_Rogue_C" (Math|Conversions|ToTransform(Vector) _output) "AdjustIfPossibleButAlwaysSpawn" self 0)))
  (Development|PrintString "Fini a liste"))

(event EventBeginPlay
  (bind _outactors (Actor|GetAllActorsOfClass "/Game/Blueprints/Grid/BP_Grid.BP_Grid_C"))
  (Variables|Default|SetGrid (Utilities|Array|Get(acopy) _outactors)))

(event EventTick
  (params (DeltaSeconds :type Float%20%28single-precision%29)))

(event Input|KeyboardEvents|Q
  (params (Key :type Key%20Structure))
  (:Pressed
    (CallFunction|TestSpawnCharacter)))

(fn ConstructionScript)