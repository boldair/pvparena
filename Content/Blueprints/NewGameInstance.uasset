(event Custom|Event_CreatSession
  (params (playerController :type Player%20Controller%20Object%20Reference))
  (bind _results (|FindSessionsAdvanced playerController 1000 false "AllServers" 0 true false false)
    (:then
      (Development|PrintString "searching"))
    (:OnSuccess
      (Variables|Default|SetFoundSessions _results)
      (Development|PrintString "Fini de chercher")
      (Development|PrintString (Utilities|String|ToString(Integer) (Utilities|Array|Length (Variables|Default|GetFoundSessions))))
      (|AdvancedSession 0 playerController 2 2 false true false true true false true false true
        (:OnSuccess
          (Development|PrintString "FINI DE CREATE SESSION")
          (Game|OpenLevel(byName) "PathfindingLevel" true "listen"))))))

(event Custom|Event_JoinSession
  (params (playerControllezr :type Player%20Controller%20Object%20Reference))
  (bind _results (|FindSessionsAdvanced playerControllezr 15 false "AllServers" 0 false false false)
    (:then
      (Development|PrintString "searching"))
    (:OnSuccess
      (Variables|Default|SetFoundSessions _results)
      (for _array_element (Variables|Default|GetFoundSessions)
        _)
      (bind _output_get (Variables|Default|SetActiveSession _array_element))
      (if (Class|AdvancedSessionsLibrary|IsValidSession _output_get)
        (|JoinSession (Game|GetPlayerController 0) _output_get
          (:OnSuccess
            (Development|PrintString "successload"))
          (:OnFailure
            (Development|PrintString "failedlo")))))))